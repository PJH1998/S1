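; Sliding door gimmick that plays a reveal sequence for PuzzleRoom001 when its activation fires.
; BeginPlay prepares the door sequence through the S1 sequence manager and binds the open handler to the cosmetic activation event.
; The handler disables player 0's input, plays the sequence and blends the view to a tag-found reveal camera.
; Sequence and camera tags are hardcoded to that room, and this graph never restores input or view.
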(event Custom|HandleOpenDoor
  (bind _returnvalue (Game|GetPlayerController 0))
  (Utilities|IsValid _returnvalue
    (:Is%20Valid
      (Input|DisableInput _returnvalue _returnvalue)
      (Class|S1SequenceManager|PlaySequencebyTag (Subsystems|GetS1SequenceManager) "(TagName=\"Sequence.Door.PuzzleRoom001\")")
      (bind _outactors (Actor|GetAllActorswithTag "RevealCamera_PuzzleRoom001"))
      (Utilities|IsValid (Utilities|Array|Get(acopy) _outactors)
        (:Is%20Valid
          (Game|Player|SetViewTargetwithBlend _returnvalue (Utilities|Array|Get(acopy) _outactors) 0.5 "VTBlend_Linear" 0.0 false))
        (:Is%20Not%20Valid
          (Development|PrintString "RevealCamera Is Not Vaild"))))))

(event EventBeginPlay
  (Class|S1SequenceManager|PrepareSequence (Subsystems|GetS1SequenceManager) "(TagName=\"Sequence.Door.PuzzleRoom001\")")
  (EventDispatchers|BindEventtoOnActivatedCosmetic (delegate Custom|HandleOpenDoor)))

(event Collision|EventActorBeginOverlap
  (params (OtherActor :type Actor%20Object%20Reference)))

(event EventTick
  (params (DeltaSeconds :type Float%20%28single-precision%29)))

(fn ConstructionScript)