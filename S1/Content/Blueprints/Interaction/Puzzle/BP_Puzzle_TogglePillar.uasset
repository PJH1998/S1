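; BP_Puzzle_TogglePillar is a toggle-pillar puzzle actor that reacts to its completion by advancing a quest.
; BeginPlay binds separate gameplay and cosmetic handlers, labeled server and client, to the inherited completion and cosmetic-activation events.
; The gameplay handler adds progress to the Stage01 OpenDoor quest through S1QuestManager.
; The cosmetic handler shows a quest-cleared announcement through the first player controller's S1UIManager.
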(event Custom|HandlePuzzleCompleted
  ;[0.15 0.15 0.15 0.5] Server
  (Class|S1QuestManager|AddQuestProgress (Subsystems|GetS1QuestManager) "(TagName=\"Quest.Stage01.OpenDoor\")" 1))

(event Custom|HandlePuzzleCompleted_Cosmetic
  (bind _returnvalue (Game|GetPlayerController 0))
  (bind _returnvalue_2 (Subsystems|GetS1UIManager _returnvalue))
  ;[0.15 0.15 0.15 0.5] Client
  (Utilities|IsValid _returnvalue
    (:Is%20Valid
      (Utilities|IsValid _returnvalue_2
        (:Is%20Valid
          (Class|S1UIManager|ShowAnnounce _returnvalue_2 (GameplayTags|MakeLiteralGameplayTag "(TagName=\"UI.Icon.Announce.QuestCleared\")")))))))

(event EventBeginPlay
  ;[0.15 0.15 0.15 0.5] Server
  (EventDispatchers|BindEventtoOnPuzzleCompleted (delegate Custom|HandlePuzzleCompleted))
  ;[0.15 0.15 0.15 0.5] Client
  (EventDispatchers|BindEventtoOnActivatedCosmetic (delegate Custom|HandlePuzzleCompleted_Cosmetic)))

(event Collision|EventActorBeginOverlap
  (params (OtherActor :type Actor%20Object%20Reference))
  ;[0.15 0.15 0.15 0.5] Comment
)

(event EventTick
  (params (DeltaSeconds :type Float%20%28single-precision%29))
  ;[0.15 0.15 0.15 0.5] Comment
)

(fn ConstructionScript)